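; ObjectManager routes player interactions with Scene 1 inspiration objects (sword, mask, tower, penin, ticket) to their dialogue.
; InteractWithObject matches the actor's object name and fires the matching interaction event.
; Each event launches that object's dialogue table and audio through the DialogueManager, then sets its progress flag on Scene1.
; The construction script caches the DialogueManager, SceneManager and its Scene1 reference via GetActorOfClass.
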(event `Interaction_Inspi_Sword`
  ;[0 1 0.4977] Scene 1 inspirational interactions
  (`/Game/Assets/Blueprints/Dialogues/DialogueManager.Dialogue Launcher` (`self.DialogueManager`) "/Game/Assets/Blueprints/Dialogues/S1P1_Inspi_Sword.S1P1_Inspi_Sword" "/Game/FMOD/Events/Scene_1/S1P1_Inspi_Sword.S1P1_Inspi_Sword")
  (set `/Game/Assets/Blueprints/Scenes/Scene1.S1P1_Inspi_Sword` true (`self.Scene 1`)))

(event `Interaction_Inspi_Mask`
  ;[0 1 0.4977] Scene 1 inspirational interactions
  (`/Game/Assets/Blueprints/Dialogues/DialogueManager.Dialogue Launcher` (`self.DialogueManager`) "/Game/Assets/Blueprints/Dialogues/S1P1_Inspi_Mask.S1P1_Inspi_Mask" "/Game/FMOD/Events/Scene_1/S1P1_Inspi_Mask.S1P1_Inspi_Mask")
  (set `/Game/Assets/Blueprints/Scenes/Scene1.S1P1_Inspi_Mask` true (`self.Scene 1`)))

(event `Interaction_Inspi_Tower`
  ;[0 1 0.4977] Scene 1 inspirational interactions
  (`/Game/Assets/Blueprints/Dialogues/DialogueManager.Dialogue Launcher` (`self.DialogueManager`) "/Game/Assets/Blueprints/Dialogues/S1P1_Inspi_Tower.S1P1_Inspi_Tower" "/Game/FMOD/Events/Scene_1/S1P1_Inspi_Tower.S1P1_Inspi_Tower")
  (set `/Game/Assets/Blueprints/Scenes/Scene1.S1P1_Inspi_Tower` true (`self.Scene 1`)))

(event `Interaction_Inspi_Penin`
  ;[0 1 0.4977] Scene 1 inspirational interactions
  (`/Game/Assets/Blueprints/Dialogues/DialogueManager.Dialogue Launcher` (`self.DialogueManager`) "/Game/Assets/Blueprints/Dialogues/S1P1_Inspi_Penin.S1P1_Inspi_Penin" "/Game/FMOD/Events/Scene_1/S1P1_Inspi_Penin.S1P1_Inspi_Penin")
  (set `/Game/Assets/Blueprints/Scenes/Scene1.S1P1_Inspi_Penin` true (`self.Scene 1`)))

(event `Interaction_Inspi_Ticket`
  ;[0 1 0.4977] Scene 1 inspirational interactions
  (`/Game/Assets/Blueprints/Dialogues/DialogueManager.Dialogue Launcher` (`self.DialogueManager`) "/Game/Assets/Blueprints/Dialogues/S1P1_Inspi_Ticket.S1P1_Inspi_Ticket" "/Game/FMOD/Events/Scene_1/S1P1_Inspi_Ticket.S1P1_Inspi_Ticket")
  (set `/Game/Assets/Blueprints/Scenes/Scene1.S1P1_Inspi_Ticket` true (`self.Scene 1`)))

(fn `InteractWithObject`
  (params (ObjectActor :type "Actor Object Reference"))
  (switch `name` (`KismetStringLibrary.Conv_StringToName` (`KismetSystemLibrary.GetObjectName` ObjectActor))
    (:`Sword`
      (`self.Interaction_Inspi_Sword`))
    (:`Mask`
      (`self.Interaction_Inspi_Mask`))
    (:`Penin`
      (`self.Interaction_Inspi_Penin`))
    (:`Tower`
      (`self.Interaction_Inspi_Tower`))
    (:`Ticket`
      (`self.Interaction_Inspi_Ticket`))))

(fn `UserConstructionScript`
  (bind _returnvalue (`GameplayStatics.GetActorOfClass` "/Game/Assets/Blueprints/Scenes/SceneManager.SceneManager_C"))
  (bind _output_get (set `self.SceneManager` _returnvalue))
  (set `self.Scene 1` (`/Game/Assets/Blueprints/Scenes/SceneManager.Scene1` _output_get))
  (bind _returnvalue_2 (`GameplayStatics.GetActorOfClass` "/Game/Assets/Blueprints/Dialogues/DialogueManager.DialogueManager_C"))
  (set `self.DialogueManager` _returnvalue_2))