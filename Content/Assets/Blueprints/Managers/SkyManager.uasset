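; Sky manager that shifts the level's lighting from day to dawn or night by rotating the directional light.
; BeginPlay caches the scene manager, sky sphere and first directional light, then applies the day rotation.
; One-shot SetDawn and SetNight set a target rotation, which Tick approaches in fixed per-axis steps, independent of delta time, until within tolerance.
; Each step teleports the sun to the new rotation and refreshes the sky sphere material.
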(event `self.ReceiveBeginPlay`
  (bind _day_rotation (`self.Day_Rotation`))
  (bind _returnvalue (`GameplayStatics.GetActorOfClass` "/Game/Assets/Blueprints/Scenes/SceneManager.SceneManager_C"))
  (set `self.SceneManager` _returnvalue)
  (bind _returnvalue_2 (`GameplayStatics.GetActorOfClass` "/Engine/EngineSky/BP_Sky_Sphere.BP_Sky_Sphere_C"))
  (set `self.Sky_Atmosphere` _returnvalue_2)
  (bind _outactors (`GameplayStatics.GetAllActorsOfClass` "/Script/Engine.DirectionalLight"))
  (if (> (`KismetArrayLibrary.Array_Length` _outactors) 0)
    (set `self.Sun` (`|GetArrayItem` _outactors))
    (`self.Set_Time` _day_rotation)
    (set `self.ActualRotation` _day_rotation)))

(event `self.ReceiveTick`
  (params (DeltaSeconds :type "Float (single-precision)"))
  (if (`self.ChangeRotation`)
    (`self.TimeTransition`)))

(fn `FloatTransition`
  (params (ActualFloat :type "Float (double-precision)") (NewFloat :type "Float (double-precision)"))
  (returns (`UpdatedFloat ` :type "Float (double-precision)"))
  (locals (UpdatedVar :type "Float (double-precision)"))
  (set `local.UpdatedVar` ActualFloat)
  (if (> ActualFloat NewFloat)
    (set `local.UpdatedVar` (- ActualFloat 0.025))
    (elif (< ActualFloat NewFloat)
      (set `local.UpdatedVar` (+ ActualFloat 0.025))))
  (return (`local.UpdatedVar`)))

(fn `Set_Dawn`
  (if (not (`self.DawnSet`))
    (set `self.NewRotation` (`self.Dawn_Rotation`))
    (set `self.ChangeRotation` true)
    (set `self.DawnSet` true)))

(fn `Set_Night`
  (if (not (`self.NightSet`))
    (set `self.NewRotation` (`self.Night_Rotation`))
    (set `self.ChangeRotation` true)
    (set `self.NightSet` true)))

(fn `Set_Time`
  (params (Time :type "Rotator Structure"))
  (bind _sun (`self.Sun`))
  (`self.K2_SetActorTransform` _sun (`KismetMathLibrary.MakeTransform` (.location (`self.GetTransform` _sun)) Time (.scale (`self.GetTransform` _sun))) false true)
  (`/Engine/EngineSky/BP_Sky_Sphere.RefreshMaterial` (`self.Sky_Atmosphere`)))

(fn `UserConstructionScript`)