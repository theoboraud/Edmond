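; Event manager that routes interactions with named scene objects to their event data in SceneManager.
; SelectObjectByName maps an object's display name to an event calling InteractWithEvent, which launches narrative or inspiration dialogue through DialogueManager with sound cues at SoundManager volumes.
; Played states are written back by reference, and playing narrative unlocks inspiration.
; Every Tick sets active objects' interaction mode from those flags, disabling them during dialogue.
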(event `self.ReceiveBeginPlay`
  (bind _returnvalue (`GameplayStatics.GetActorOfClass` "/Game/Assets/Blueprints/Scenes/SceneManager.SceneManager_C"))
  (set `self.SceneManager` _returnvalue)
  (bind _returnvalue_2 (`GameplayStatics.GetActorOfClass` "/Game/Assets/Blueprints/Dialogues/DialogueManager.DialogueManager_C"))
  (set `self.DialogueManager` _returnvalue_2)
  (bind _returnvalue_3 (`GameplayStatics.GetActorOfClass` "/Game/Assets/Blueprints/Managers/SoundManager.SoundManager_C"))
  (set `self.SoundManager` _returnvalue_3))

(event `self.ReceiveTick`
  (params (DeltaSeconds :type "Float (single-precision)"))
  (`self.SetAllObjects_CanPlay`))

(event `Interaction_Helmet`
  ;[1 1 1] Scene 2 objects
  (`self.InteractWithEvent` (`/Game/Assets/Blueprints/Scenes/Scene_2.Helmet` (`/Game/Assets/Blueprints/Scenes/SceneManager.Scene2` (`self.SceneManager`)))))

(event `Interaction_Inspi_Sword`
  ;[0 1 0.4977] Scene 1 objects
  (`self.InteractWithEvent` (`/Game/Assets/Blueprints/Scenes/Scene_1.Sword` (`/Game/Assets/Blueprints/Scenes/SceneManager.Scene1` (`self.SceneManager`)))))

(event `Interaction_Sticker`
  ;[1 1 1] Scene 3 objects
  (`self.InteractWithEvent` (`/Game/Assets/Blueprints/Scenes/Scene_3.Sticker` (`/Game/Assets/Blueprints/Scenes/SceneManager.Scene3` (`self.SceneManager`)))))

(event `Interaction_Apo`
  ;[1 1 1] Scene 2 objects
  (`self.InteractWithEvent` (`/Game/Assets/Blueprints/Scenes/Scene_2.Apo` (`/Game/Assets/Blueprints/Scenes/SceneManager.Scene2` (`self.SceneManager`)))))

(event `Interaction_Picture`
  ;[1 1 1] Scene 3 objects
  (`self.InteractWithEvent` (`/Game/Assets/Blueprints/Scenes/Scene_3.Picture` (`/Game/Assets/Blueprints/Scenes/SceneManager.Scene3` (`self.SceneManager`)))))

(event `Interaction_Inspi_Mask`
  ;[0 1 0.4977] Scene 1 objects
  (`self.InteractWithEvent` (`/Game/Assets/Blueprints/Scenes/Scene_1.Mask` (`/Game/Assets/Blueprints/Scenes/SceneManager.Scene1` (`self.SceneManager`)))))

(event `Interaction_Foil`
  ;[1 1 1] Scene 2 objects
  (`self.InteractWithEvent` (`/Game/Assets/Blueprints/Scenes/Scene_2.Foil` (`/Game/Assets/Blueprints/Scenes/SceneManager.Scene2` (`self.SceneManager`)))))

(event `Interaction_Underwear`
  ;[1 1 1] Scene 3 objects
  (`self.InteractWithEvent` (`/Game/Assets/Blueprints/Scenes/Scene_3.Underwear` (`/Game/Assets/Blueprints/Scenes/SceneManager.Scene3` (`self.SceneManager`)))))

(event `Interaction_Medocs`
  ;[1 1 1] Scene 2 objects
  (`self.InteractWithEvent` (`/Game/Assets/Blueprints/Scenes/Scene_2.Medocs` (`/Game/Assets/Blueprints/Scenes/SceneManager.Scene2` (`self.SceneManager`)))))

(event `Interaction_Inspi_Tower`
  ;[0 1 0.4977] Scene 1 objects
  (`self.InteractWithEvent` (`/Game/Assets/Blueprints/Scenes/Scene_1.Tower` (`/Game/Assets/Blueprints/Scenes/SceneManager.Scene1` (`self.SceneManager`)))))

(event `Interaction_Number`
  ;[1 1 1] Scene 3 objects
  (`self.InteractWithEvent` (`/Game/Assets/Blueprints/Scenes/Scene_3.Number` (`/Game/Assets/Blueprints/Scenes/SceneManager.Scene3` (`self.SceneManager`)))))

(event `Interaction_Stetson`
  ;[1 1 1] Scene 2 objects
  (`self.InteractWithEvent` (`/Game/Assets/Blueprints/Scenes/Scene_2.Stetson` (`/Game/Assets/Blueprints/Scenes/SceneManager.Scene2` (`self.SceneManager`)))))

(event `Interaction_Inspi_Penin`
  ;[0 1 0.4977] Scene 1 objects
  (`self.InteractWithEvent` (`/Game/Assets/Blueprints/Scenes/Scene_1.Penin` (`/Game/Assets/Blueprints/Scenes/SceneManager.Scene1` (`self.SceneManager`)))))

(event `Interaction_Inspi_Ticket`
  ;[0 1 0.4977] Scene 1 objects
  (`self.InteractWithEvent` (`/Game/Assets/Blueprints/Scenes/Scene_1.Ticket` (`/Game/Assets/Blueprints/Scenes/SceneManager.Scene1` (`self.SceneManager`)))))

(event `Moon`
  (`self.InteractWithEvent` (`/Game/Assets/Blueprints/Scenes/Scene_5.Moon` (`/Game/Assets/Blueprints/Scenes/SceneManager.Scene5` (`self.SceneManager`)))))

(event `Interaction_Bowl`
  ;[1 1 1] Narrative objects
  (`KismetSystemLibrary.PrintString` "Hello")
  (`self.InteractWithEvent` (`/Game/Assets/Blueprints/Scenes/Scene_Narrative.Bowl` (`/Game/Assets/Blueprints/Scenes/SceneManager.Scene_Narrative` (`self.SceneManager`)))))

(event `Feather`
  (`self.InteractWithEvent` (`/Game/Assets/Blueprints/Scenes/Scene_5.Feather` (`/Game/Assets/Blueprints/Scenes/SceneManager.Scene5` (`self.SceneManager`)))))

(event `Interaction_Box`
  ;[1 1 1] Narrative objects
  (`self.InteractWithEvent` (`/Game/Assets/Blueprints/Scenes/Scene_Narrative.Box` (`/Game/Assets/Blueprints/Scenes/SceneManager.Scene_Narrative` (`self.SceneManager`)))))

(event `Question`
  (`self.InteractWithEvent` (`/Game/Assets/Blueprints/Scenes/Scene_5.Question` (`/Game/Assets/Blueprints/Scenes/SceneManager.Scene5` (`self.SceneManager`)))))

(event `Interaction_Poem`
  ;[1 1 1] Narrative objects
  (`self.InteractWithEvent` (`/Game/Assets/Blueprints/Scenes/Scene_Narrative.Poem` (`/Game/Assets/Blueprints/Scenes/SceneManager.Scene_Narrative` (`self.SceneManager`)))))

(event `Heart`
  (`self.InteractWithEvent` (`/Game/Assets/Blueprints/Scenes/Scene_5.Heart` (`/Game/Assets/Blueprints/Scenes/SceneManager.Scene5` (`self.SceneManager`)))))

(event `Interaction_Class`
  ;[1 1 1] Narrative objects
  (`self.InteractWithEvent` (`/Game/Assets/Blueprints/Scenes/Scene_Narrative.Class` (`/Game/Assets/Blueprints/Scenes/SceneManager.Scene_Narrative` (`self.SceneManager`)))))

(event `Pillow`
  (`self.InteractWithEvent` (`/Game/Assets/Blueprints/Scenes/Scene_5.Pillow` (`/Game/Assets/Blueprints/Scenes/SceneManager.Scene5` (`self.SceneManager`)))))

(event `Interaction_Sign`
  ;[1 1 1] Narrative objects
  (`self.InteractWithEvent` (`/Game/Assets/Blueprints/Scenes/Scene_Narrative.Sign` (`/Game/Assets/Blueprints/Scenes/SceneManager.Scene_Narrative` (`self.SceneManager`)))))

(event `Stairs`
  (`self.InteractWithEvent` (`/Game/Assets/Blueprints/Scenes/Scene_5.Stairs` (`/Game/Assets/Blueprints/Scenes/SceneManager.Scene5` (`self.SceneManager`)))))

(event `Interaction_Certif`
  ;[1 1 1] Narrative objects
  (`self.InteractWithEvent` (`/Game/Assets/Blueprints/Scenes/Scene_Narrative.Certif` (`/Game/Assets/Blueprints/Scenes/SceneManager.Scene_Narrative` (`self.SceneManager`)))))

(event `Watch`
  (`self.InteractWithEvent` (`/Game/Assets/Blueprints/Scenes/Scene_5.Watch` (`/Game/Assets/Blueprints/Scenes/SceneManager.Scene5` (`self.SceneManager`)))))

(event `Interaction_Degree`
  ;[1 1 1] Narrative objects
  (`self.InteractWithEvent` (`/Game/Assets/Blueprints/Scenes/Scene_Narrative.Degree` (`/Game/Assets/Blueprints/Scenes/SceneManager.Scene_Narrative` (`self.SceneManager`)))))

(event `Crown`
  (`self.InteractWithEvent` (`/Game/Assets/Blueprints/Scenes/Scene_5.Crown` (`/Game/Assets/Blueprints/Scenes/SceneManager.Scene5` (`self.SceneManager`)))))

(event `Interaction_Check`
  ;[1 1 1] Narrative objects
  (`self.InteractWithEvent` (`/Game/Assets/Blueprints/Scenes/Scene_Narrative.Check` (`/Game/Assets/Blueprints/Scenes/SceneManager.Scene_Narrative` (`self.SceneManager`)))))

(event `Sun`
  (`self.InteractWithEvent` (`/Game/Assets/Blueprints/Scenes/Scene_5.Sun` (`/Game/Assets/Blueprints/Scenes/SceneManager.Scene5` (`self.SceneManager`)))))

(event `Micro`
  (`self.InteractWithEvent` (`/Game/Assets/Blueprints/Scenes/Scene_5.Micro` (`/Game/Assets/Blueprints/Scenes/SceneManager.Scene5` (`self.SceneManager`)))))

(event `Flowers`
  (`self.InteractWithEvent` (`/Game/Assets/Blueprints/Scenes/Scene_5.Flowers` (`/Game/Assets/Blueprints/Scenes/SceneManager.Scene5` (`self.SceneManager`)))))

(event `Feather2`
  (`self.InteractWithEvent` (`/Game/Assets/Blueprints/Scenes/Scene_5.Feather2` (`/Game/Assets/Blueprints/Scenes/SceneManager.Scene5` (`self.SceneManager`)))))

(event `Bell`
  (`self.InteractWithEvent` (`/Game/Assets/Blueprints/Scenes/Scene_5.Bell` (`/Game/Assets/Blueprints/Scenes/SceneManager.Scene5` (`self.SceneManager`)))))

(fn `Get Idea From Class`
  (params (ObjectClass :type "/Game/Assets/Blueprints/Objects/InteractableObject Class Reference"))
  (returns (Idea :type String))
  (bind _exec (`/Game/Assets/Blueprints/Scenes/SceneManager.GetAllActiveObjects` (`self.SceneManager`)))
  (for _array_element _exec
    (bind (_objectclass _canplay_narra _played_narra _audio_narra _subtitle_narra _canplay_inspi _played_inspi _audio_inspi _subtitle_inspi _idea_inspi) (break `/Game/Assets/Blueprints/Dialogues/EventData` _array_element))
    (if (== _objectclass ObjectClass)
      (return _idea_inspi))))

(fn `InteractWithEvent`
  (params (EventData :type "/Game/Assets/Blueprints/Dialogues/EventData Structure (by ref)"))
  (bind (_objectclass _canplay_narra _played_narra _audio_narra _subtitle_narra _canplay_inspi _played_inspi _audio_inspi _subtitle_inspi _idea_inspi) (break `/Game/Assets/Blueprints/Dialogues/EventData` EventData))
  (bind _dialoguemanager (`self.DialogueManager`))
  (bind _scenecount (`/Game/Assets/Blueprints/Scenes/SceneManager.SceneCount` (`self.SceneManager`)))
  (if (and _canplay_narra (not _played_narra))
    (`/Game/Assets/Blueprints/Dialogues/DialogueManager.Dialogue Launcher` _dialoguemanager _audio_narra _subtitle_narra)
    (if (`KismetSystemLibrary.IsValidClass` _objectclass)
      (bind _returnvalue (`FMODBlueprintStatics.PlayEvent2D` "/Game/FMOD/Events/Feedbacks/Intera_narra.Intera_narra"))
      (`FMODBlueprintStatics.EventInstanceSetVolume` _returnvalue (`/Game/Assets/Blueprints/Managers/SoundManager.Volume_InteractionNarra` (`self.SoundManager`))))
    (`|VariableSetRef` EventData (make `/Game/Assets/Blueprints/Dialogues/EventData` _objectclass false true _audio_narra _subtitle_narra true _played_inspi _audio_inspi _subtitle_inspi _idea_inspi))
    (return)
    (elif (and _canplay_inspi (not _played_inspi))
      (`/Game/Assets/Blueprints/Dialogues/DialogueManager.Dialogue Launcher` _dialoguemanager _audio_inspi _subtitle_inspi)
      (if (and (>= _scenecount 2) (<= _scenecount 4))
        (bind _returnvalue_2 (`FMODBlueprintStatics.PlayEvent2D` "/Game/FMOD/Events/Ambience/Music/Inspi/Inspi.Inspi"))
        (`FMODBlueprintStatics.EventInstanceSetVolume` _returnvalue_2 (`/Game/Assets/Blueprints/Managers/SoundManager.Volume_InteractionInspi` (`self.SoundManager`))))
      (`|VariableSetRef` EventData (make `/Game/Assets/Blueprints/Dialogues/EventData` _objectclass _canplay_narra _played_narra _audio_narra _subtitle_narra false true _audio_inspi _subtitle_inspi _idea_inspi))
      (return))))

(fn `SelectObjectByName`
  (params (ObjectActor :type "Actor Object Reference"))
  (bind _asinteractable_object (cast `/Game/Assets/Blueprints/Objects/InteractableObject` ObjectActor))
  (if (and (`self.DialogueNotInPlay`) (`/Game/Assets/Blueprints/Objects/InteractableObject.CanInteract` _asinteractable_object))
    (switch `name` (`KismetStringLibrary.Conv_StringToName` (`KismetSystemLibrary.GetDisplayName` _asinteractable_object))
      (:`Sword`
        (`self.Interaction_Inspi_Sword`))
      (:`Mask`
        (`self.Interaction_Inspi_Mask`))
      (:`Peninsula`
        (`self.Interaction_Inspi_Penin`))
      (:`Tower`
        (`self.Interaction_Inspi_Tower`))
      (:`Ticket`
        (`self.Interaction_Inspi_Ticket`))
      (:`Helmet`
        (`self.Interaction_Helmet`))
      (:`Foil`
        (`self.Interaction_Foil`))
      (:`Apo`
        (`self.Interaction_Apo`))
      (:`Medocs`
        (`self.Interaction_Medocs`))
      (:`Stetson`
        (`self.Interaction_Stetson`))
      (:`Sticker`
        (`self.Interaction_Sticker`))
      (:`Number`
        (`self.Interaction_Number`))
      (:`Underwear`
        (`self.Interaction_Underwear`))
      (:`Picture`
        (`self.Interaction_Picture`))
      (:`Bowl`
        (`self.Interaction_Bowl`))
      (:`Box`
        (`self.Interaction_Box`))
      (:`Certif`
        (`self.Interaction_Certif`))
      (:`Class`
        (`self.Interaction_Class`))
      (:`Degree`
        (`self.Interaction_Degree`))
      (:`Sign`
        (`self.Interaction_Sign`))
      (:`Poem`
        (`self.Interaction_Poem`))
      (:`Check`
        (`self.Interaction_Check`))
      (:`Moon`
        (`self.Moon`))
      (:`Feather`
        (`self.Feather`))
      (:`Question`
        (`self.Question`))
      (:`Heart`
        (`self.Heart`))
      (:`Pillow`
        (`self.Pillow`))
      (:`Stairs`
        (`self.Stairs`))
      (:`Watch`
        (`self.Watch`))
      (:`Crown`
        (`self.Crown`))
      (:`Sun`
        (`self.Sun`))
      (:`Micro`
        (`self.Micro`))
      (:`Flowers`
        (`self.Flowers`))
      (:`Feather2`
        (`self.Feather2`))
      (:`Bell`
        (`self.Bell`)))))

(fn `SetAllObjects_CanPlay`
  (locals (CanPlay :type Boolean))
  (bind _exec (`/Game/Assets/Blueprints/Scenes/SceneManager.GetAllActiveObjects` (`self.SceneManager`)))
  (for _array_element _exec
    (if (not (`self.DialogueNotInPlay`))
      (bind (_objectclass _canplay_narra _played_narra _audio_narra _subtitle_narra _canplay_inspi _played_inspi) (break `/Game/Assets/Blueprints/Dialogues/EventData` _array_element))
      (`self.SetObject_CanPlay` _objectclass)
      (elif (and _canplay_narra (not _played_narra))
        (`self.SetObject_CanPlay` _objectclass _canplay_narra)
        (elif (and _canplay_inspi (not _played_inspi))
          (`self.SetObject_CanPlay` _objectclass false _canplay_inspi))))))

(fn `SetObject_CanPlay`
  (params (Object :type "Actor Class Reference (by ref)") (CanPlay_Narra :type Boolean) (CanPlay_Inspi :type Boolean))
  (bind _returnvalue (`GameplayStatics.GetActorOfClass` Object))
  (bind _asinteractable_object (cast `/Game/Assets/Blueprints/Objects/InteractableObject` _returnvalue)
    (:`then`
      (if CanPlay_Narra
        (`/Game/Assets/Blueprints/Objects/InteractableObject.Set_Interact_Narra` _asinteractable_object)
        (elif CanPlay_Inspi
          (`/Game/Assets/Blueprints/Objects/InteractableObject.Set_Interact_Inspi` _asinteractable_object)
          (else
            (`/Game/Assets/Blueprints/Objects/InteractableObject.Set_NoInteract` _asinteractable_object)))))
    (:`CastFailed`
      (`KismetSystemLibrary.PrintString` (`KismetStringLibrary.Concat_StrStr` (`KismetSystemLibrary.GetClassDisplayName` Object) " is not interactable")))))

(fn `UserConstructionScript`)