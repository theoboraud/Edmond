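; InteractableObject is an interactable object Blueprint that tracks whether it can be interacted with and which outline material applies.
; Three setters store the Narra, Inspi or empty material in a variable and update the CanInteract flag.
; The Inspi and no-interact setters also toggle the Outline component's visibility through a helper, while the Narra setter leaves visibility unchanged.
; Its event graph and construction script are empty.
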(event `self.ReceiveBeginPlay`)

(fn `Set_Interact_Inspi`
  (set `self.Material` "/Game/Assets/Blueprints/Inspi_Outline.Inspi_Outline")
  (bind _output_get (set `self.CanInteract` true))
  (`self.SetOutlineVisibility` _output_get))

(fn `Set_Interact_Narra`
  (set `self.Material` "/Game/Assets/Blueprints/Narra_Outline.Narra_Outline")
  (set `self.CanInteract` true))

(fn `Set_NoInteract`
  (set `self.Material` null)
  (bind _output_get (set `self.CanInteract` false))
  (`self.SetOutlineVisibility` _output_get))

(fn `SetOutlineVisibility`
  (params (IsVisible :type Boolean))
  (`SceneComponent.SetVisibility` (`self.Outline`) IsVisible false))

(fn `UserConstructionScript`)