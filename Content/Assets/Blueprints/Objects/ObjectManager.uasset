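; Manager actor for Scene 1's five inspiration objects, playing each one's dialogue when the player interacts with it.
; InteractWithObject routes by actor display name to an event that checks the scene flag, launches dialogue with audio, records the interaction and disables the object.
; The construction script caches SceneManager and DialogueManager via GetActorOfClass.
; SetScene is an empty stub, and CanInteractWithObject's InteractionInPlay check is left unwired.
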(event `self.ReceiveBeginPlay`)

(event `Interaction_Inspi_Sword`
  ;[0 1 0.4977] Scene 1 inspirational interactions
  (if (`self.CanInteractWithObject` (`/Game/Assets/Blueprints/Scenes/Scene1.CanInteract_Sword` (`self.Scene 1`)))
    (`/Game/Assets/Blueprints/Dialogues/DialogueManager.Dialogue Launcher` (`self.DialogueManager`) "/Game/Assets/Blueprints/Dialogues/Subtitles/Scene1/S1P1_Inspi_Sword.S1P1_Inspi_Sword" "/Game/FMOD/Events/Scene_1/S1P1_Inspi_Sword.S1P1_Inspi_Sword")
    (set `/Game/Assets/Blueprints/Scenes/Scene1.Interacted_Sword` true (`self.Scene 1`))
    (`self.SetObjectInteractable` "/Game/Assets/Blueprints/Objects/Sword.Sword_C")))

(event `Interaction_Inspi_Mask`
  ;[0 1 0.4977] Scene 1 inspirational interactions
  (if (`self.CanInteractWithObject` (`/Game/Assets/Blueprints/Scenes/Scene1.CanInteract_Mask` (`self.Scene 1`)))
    (`/Game/Assets/Blueprints/Dialogues/DialogueManager.Dialogue Launcher` (`self.DialogueManager`) "/Game/Assets/Blueprints/Dialogues/Subtitles/Scene1/S1P1_Inspi_Mask.S1P1_Inspi_Mask" "/Game/FMOD/Events/Scene_1/S1P1_Inspi_Mask.S1P1_Inspi_Mask")
    (set `/Game/Assets/Blueprints/Scenes/Scene1.Interacted_Mask` true (`self.Scene 1`))
    (`self.SetObjectInteractable` "/Game/Assets/Blueprints/Objects/Mask.Mask_C")))

(event `Interaction_Inspi_Tower`
  ;[0 1 0.4977] Scene 1 inspirational interactions
  (if (`self.CanInteractWithObject` (`/Game/Assets/Blueprints/Scenes/Scene1.CanInteract_Tower` (`self.Scene 1`)))
    (`/Game/Assets/Blueprints/Dialogues/DialogueManager.Dialogue Launcher` (`self.DialogueManager`) "/Game/Assets/Blueprints/Dialogues/Subtitles/Scene1/S1P1_Inspi_Tower.S1P1_Inspi_Tower" "/Game/FMOD/Events/Scene_1/S1P1_Inspi_Tower.S1P1_Inspi_Tower")
    (set `/Game/Assets/Blueprints/Scenes/Scene1.Interacted_Tower` true (`self.Scene 1`))
    (`self.SetObjectInteractable` "/Game/Assets/Blueprints/Objects/Tower.Tower_C")))

(event `Interaction_Inspi_Penin`
  ;[0 1 0.4977] Scene 1 inspirational interactions
  (if (`self.CanInteractWithObject` (`/Game/Assets/Blueprints/Scenes/Scene1.CanInteract_Penin` (`self.Scene 1`)))
    (`/Game/Assets/Blueprints/Dialogues/DialogueManager.Dialogue Launcher` (`self.DialogueManager`) "/Game/Assets/Blueprints/Dialogues/Subtitles/Scene1/S1P1_Inspi_Penin.S1P1_Inspi_Penin" "/Game/FMOD/Events/Scene_1/S1P1_Inspi_Penin.S1P1_Inspi_Penin")
    (set `/Game/Assets/Blueprints/Scenes/Scene1.Interacted_Penin` true (`self.Scene 1`))
    (`self.SetObjectInteractable` "/Game/Assets/Blueprints/Objects/Peninsula.Peninsula_C")))

(event `Interaction_Inspi_Ticket`
  ;[0 1 0.4977] Scene 1 inspirational interactions
  (if (`self.CanInteractWithObject` (`/Game/Assets/Blueprints/Scenes/Scene1.CanInteract_Ticket` (`self.Scene 1`)))
    (`/Game/Assets/Blueprints/Dialogues/DialogueManager.Dialogue Launcher` (`self.DialogueManager`) "/Game/Assets/Blueprints/Dialogues/Subtitles/Scene1/S1P1_Inspi_Ticket.S1P1_Inspi_Ticket" "/Game/FMOD/Events/Scene_1/S1P1_Inspi_Ticket.S1P1_Inspi_Ticket")
    (set `/Game/Assets/Blueprints/Scenes/Scene1.Interacted_Ticket` true (`self.Scene 1`))
    (`self.SetObjectInteractable` "/Game/Assets/Blueprints/Objects/Ticket.Ticket_C")))

(fn `InteractWithObject`
  (params (ObjectActor :type "Actor Object Reference"))
  (bind _returnvalue (`KismetSystemLibrary.GetDisplayName` ObjectActor))
  (`KismetSystemLibrary.PrintString` _returnvalue)
  (switch `name` (`KismetStringLibrary.Conv_StringToName` _returnvalue)
    (:`Sword`
      (`self.Interaction_Inspi_Sword`))
    (:`Mask`
      (`self.Interaction_Inspi_Mask`))
    (:`Peninsula`
      (`self.Interaction_Inspi_Penin`))
    (:`Tower`
      (`self.Interaction_Inspi_Tower`))
    (:`Ticket`
      (`self.Interaction_Inspi_Ticket`))))

(fn `Set Scene`
  (params (`Scene Reference` :type "UserWidget Object Reference") (`Scene Class` :type "UserWidget Class Reference")))

(fn `SetObjectInteractable`
  (params (Object :type "Actor Class Reference") (IsInteractable :type Boolean))
  (bind _returnvalue (`GameplayStatics.GetActorOfClass` Object))
  (bind _asinteractable_object (cast `/Game/Assets/Blueprints/Objects/InteractableObject` _returnvalue))
  (if IsInteractable
    (`/Game/Assets/Blueprints/Objects/InteractableObject.CanInteract` _asinteractable_object)
    (else
      (`/Game/Assets/Blueprints/Objects/InteractableObject.CannotInteract` _asinteractable_object))))

(fn `UserConstructionScript`
  (bind _returnvalue (`GameplayStatics.GetActorOfClass` "/Game/Assets/Blueprints/Scenes/SceneManager.SceneManager_C"))
  (set `self.SceneManager` _returnvalue)
  (bind _returnvalue_2 (`GameplayStatics.GetActorOfClass` "/Game/Assets/Blueprints/Dialogues/DialogueManager.DialogueManager_C"))
  (set `self.DialogueManager` _returnvalue_2)
  (set `self.InteractionInPlay` false))