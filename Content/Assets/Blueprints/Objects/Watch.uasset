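; Watch object that inherits its behavior, including outline highlighting, from a parent class.
; On BeginPlay it registers the Clock component as the outline target, turns the outline off, and hides the Cube component and its children.
; Overlap and construction only call the parent, and Tick is disabled.
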(event `self.ReceiveBeginPlay`
  (`parent.ReceiveBeginPlay`)
  (set `self.Outline` (`self.Clock`))
  (`self.SetOutlineVisibility` false)
  (`SceneComponent.SetVisibility` (`self.Cube`) false true))

(event `self.ReceiveActorBeginOverlap`
  (params (OtherActor :type "Actor Object Reference"))
  (`parent.ReceiveActorBeginOverlap` OtherActor))

(fn `UserConstructionScript`
  (`parent.UserConstructionScript`))