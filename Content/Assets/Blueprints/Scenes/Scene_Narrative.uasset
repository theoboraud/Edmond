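; Scene Blueprint for the narrative scene, controlling which of eight story objects (Check, Class, Degree, Bowl, Box, Certif, Poem, Sign) can play their dialogue.
; On BeginPlay it loads each object's event data from the Narrative_EventsData1 data table by row name.
; Once initialized, every Tick with no dialogue in play enables narration only for objects not yet played and disables Inspi playback.
; A helper can also set both flags on all objects at once.
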(event `self.ReceiveBeginPlay`
  (`self.GetDataFromEvent`))

(event `self.ReceiveTick`
  (params (DeltaSeconds :type "Float (single-precision)"))
  ;[1 1 1] Start scene if initialized
  (if (`self.Initialized`)
    ;[1 1 1] Don't do anything if a dialogue is in play
    (bind _dialoguenotinplay (`self.DialogueNotInPlay`))
    (if _dialoguenotinplay
      (`self.InitlializeCanPlay_AllObjects`))))

(fn `GetAllObjects`
  (returns (Array :type "Array of /Game/Assets/Blueprints/Dialogues/EventData Structure"))
  (return (`|MakeArray` (`self.Check`) (`self.Class`) (`self.Degree`) (`self.Bowl`) (`self.Box`) (`self.Certif`) (`self.Poem`) (`self.Sign`))))

(fn `UserConstructionScript`
  (`parent.UserConstructionScript`))