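; Scene 5 controller that sequences narration, Jeanne's dialogues and interactive objects from intro to outro.
; BeginPlay loads event rows from the Scene5_EventsData table into named variables.
; Tick waits for dialogue to finish, plays Intro2 outdoors, then steps through four object groups, each unlocking the next after one Inspi interaction.
; The outro sets EndTrigger, which flags SceneManager; Watch always stays disabled in Group 2's toggle.
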(event `self.ReceiveBeginPlay`
  (bind _returnvalue (`GameplayStatics.GetActorOfClass` "/Game/Assets/Props/Atmosphere/TriggerAtmosphere.TriggerAtmosphere_C"))
  (set `self.TriggerAtmosphere` _returnvalue)
  (bind _returnvalue_2 (`GameplayStatics.GetActorOfClass` "/Game/Assets/Props/Jeanne/Jeanne.Jeanne_C"))
  (set `self.Jeanne` _returnvalue_2)
  (`self.GetDataFromEvent`))

(event `self.ReceiveTick`
  (params (DeltaSeconds :type "Float (single-precision)"))
  ;[1 1 1] Start scene if initialized
  (if (`self.Initialized`)
    ;[1 1 1] Don't do anything if a dialogue is in play
    (bind _dialoguenotinplay (`self.DialogueNotInPlay`))
    (if _dialoguenotinplay
      ;[1 1 1] Stop here if scene 5 ended
      (if (`self.EndTrigger`)
        (set `/Game/Assets/Blueprints/Scenes/SceneManager.Scene5_EndTrigger` true (`self.SceneManager`))
        (else
          (`self.InteractionIfNotPlayed` (`self.Intro`) true)
          (bind _played_narra (`self.GetPlayed` (`self.Intro2`)))
          (if _played_narra
            (bind _array (`self.GetObjects_Group1`))
            (bind _succeeded (`self.If at Least X Played` _array 1 false true))
            (if _succeeded
              (bind _justplayed (`self.InteractionIfNotPlayed` (`self.Group1`) true))
              (`/Game/Assets/Props/Jeanne/Jeanne.LaunchJeanneDialogue` (`self.Jeanne`) (`self.Group1_Jeanne`))
              (if _justplayed
                (`self.SetCanPlay_Group1` false
                  (:`Exec `
                    (`self.SetCanPlay_Group2` false true)))
                (else
                  (bind _array_2 (`self.GetObjects_Group2`))
                  (bind _succeeded_2 (`self.If at Least X Played` _array_2 1 false true))
                  (if _succeeded_2
                    (bind _justplayed_2 (`self.InteractionIfNotPlayed` (`self.Group2`) true))
                    (`/Game/Assets/Props/Jeanne/Jeanne.LaunchJeanneDialogue` (`self.Jeanne`) (`self.Group2_Jeanne`))
                    (if _justplayed_2
                      (`self.SetCanPlay_Group2` false
                        (:`Exec `
                          (`self.SetCanPlay_Group3` false true)))
                      (else
                        (bind _array_3 (`self.GetObjects_Group3`))
                        (bind _succeeded_3 (`self.If at Least X Played` _array_3 1 false true))
                        (if _succeeded_3
                          (bind _justplayed_3 (`self.InteractionIfNotPlayed` (`self.Group3`) true))
                          (`/Game/Assets/Props/Jeanne/Jeanne.LaunchJeanneDialogue` (`self.Jeanne`) (`self.Group3_Jeanne`))
                          (if _justplayed_3
                            (`self.SetCanPlay_Group3` false
                              (:`Exec `
                                (`self.SetCanPlay_Group4` false true)))
                            (else
                              (bind _array_4 (`self.GetObjects_Group4`))
                              (bind _succeeded_4 (`self.If at Least X Played` _array_4 1 false true))
                              (if _succeeded_4
                                (bind _justplayed_4 (`self.InteractionIfNotPlayed` (`self.Group4`) true))
                                (`/Game/Assets/Props/Jeanne/Jeanne.LaunchJeanneDialogue` (`self.Jeanne`) (`self.Group4_Jeanne`))
                                (if _justplayed_4
                                  (`self.SetCanPlay_Group4` false)
                                  (else
                                    (bind _justplayed_5 (`self.InteractionIfNotPlayed` (`self.Outro`) true))
                                    (if _justplayed_5
                                      (set `self.EndTrigger` true))))))))))))))
            (elif (`/Game/Assets/Props/Atmosphere/TriggerAtmosphere.IsOutdoor` (`self.TriggerAtmosphere`))
              (bind _justplayed_6 (`self.InteractionIfNotPlayed` (`self.Intro2`) true))
              (`/Game/Assets/Props/Jeanne/Jeanne.LaunchJeanneDialogue` (`self.Jeanne`) (`self.Intro2_Jeanne`))
              (if _justplayed_6
                (`self.SetCanPlay_Group1` false true)))))))))

(fn `GetAllObjects`
  (returns (Array :type "Array of /Game/Assets/Blueprints/Dialogues/EventData Structure"))
  (locals (NewArray :type "Array of /Game/Assets/Blueprints/Dialogues/EventData Structure"))
  (bind _newarray (`local.NewArray`))
  (bind _array (`self.GetObjects_Group1`))
  (bind _array_2 (`self.GetObjects_Group2`))
  (bind _array_3 (`self.GetObjects_Group3`))
  (bind _array_4 (`self.GetObjects_Group4`))
  (`KismetArrayLibrary.Array_Append` _newarray _array)
  (`KismetArrayLibrary.Array_Append` _newarray _array_2)
  (`KismetArrayLibrary.Array_Append` _newarray _array_3)
  (`KismetArrayLibrary.Array_Append` _newarray _array_4)
  (return (`local.NewArray`)))

(fn `GetObjects_Group1`
  (returns (Array :type "Array of /Game/Assets/Blueprints/Dialogues/EventData Structure"))
  (return (`|MakeArray` (`self.Moon`) (`self.Feather`) (`self.Question`))))

(fn `GetObjects_Group2`
  (returns (Array :type "Array of /Game/Assets/Blueprints/Dialogues/EventData Structure"))
  (return (`|MakeArray` (`self.Heart`) (`self.Pillow`) (`self.Stairs`) (`self.Watch`))))

(fn `GetObjects_Group3`
  (returns (Array :type "Array of /Game/Assets/Blueprints/Dialogues/EventData Structure"))
  (return (`|MakeArray` (`self.Crown`) (`self.Sun`) (`self.Micro`))))

(fn `GetObjects_Group4`
  (returns (Array :type "Array of /Game/Assets/Blueprints/Dialogues/EventData Structure"))
  (return (`|MakeArray` (`self.Flowers`) (`self.Feather2`) (`self.Bell`))))

(fn `UserConstructionScript`
  (`parent.UserConstructionScript`))