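; Scene actor with helper functions that control when event objects can play their Narra and Inspi dialogue.
; Construction caches the DialogueManager, SceneManager and EventManager actors found in the level.
; SetCanPlay allows Narra only until played and Inspi only after Narra, then updates the EventData by reference and notifies EventManager.
; Other helpers set played flags, count played events, check for active dialogue and trigger unplayed interactions through EventManager.
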(event `self.ReceiveBeginPlay`)

(fn `DialogueNotInPlay`
  (returns (DialogueNotInPlay :type Boolean))
  (return (not (`/Game/Assets/Blueprints/Dialogues/DialogueManager.DialogueInPlay` (`self.DialogueManager`)))))

(fn `GetCanPlay`
  (params (EventData :type "/Game/Assets/Blueprints/Dialogues/EventData Structure"))
  (returns (CanPlay_Narra :type Boolean) (CanPlay_Inspi :type Boolean))
  (bind (_objectclass _canplay_narra _played_narra _audio_narra _subtitle_narra _canplay_inspi) (break `/Game/Assets/Blueprints/Dialogues/EventData` EventData))
  (return _canplay_narra _canplay_inspi))

(fn `GetPlayed`
  (params (EventData :type "/Game/Assets/Blueprints/Dialogues/EventData Structure"))
  (returns (Played_Narra :type Boolean) (Played_Inspi :type Boolean))
  (bind (_objectclass _canplay_narra _played_narra _audio_narra _subtitle_narra _canplay_inspi _played_inspi) (break `/Game/Assets/Blueprints/Dialogues/EventData` EventData))
  (return _played_narra _played_inspi))

(fn `If at Least X Played`
  (params (EventData :type "Array of /Game/Assets/Blueprints/Dialogues/EventData Structure") (X :type Integer) (Narra :type Boolean) (Inspi :type Boolean))
  (returns (Succeeded :type Boolean))
  (locals (X_Counter :type Integer) (Played_Counter :type Integer))
  (bind _returnvalue (+ (`local.Played_Counter`) 1))
  (set `local.X_Counter` X)
  (set `local.Played_Counter` 0)
  (for _array_element EventData
    (if Narra
      (bind (_objectclass _canplay_narra _played_narra _audio_narra _subtitle_narra _canplay_inspi _played_inspi) (break `/Game/Assets/Blueprints/Dialogues/EventData` _array_element))
      (if _played_narra
        (set `local.Played_Counter` _returnvalue))
      (elif Inspi
        (if _played_inspi
          (set `local.Played_Counter` _returnvalue)))))
  (return (<= (`local.X_Counter`) (`local.Played_Counter`))))

(fn `InteractionIfNotPlayed`
  (params (EventData :type "/Game/Assets/Blueprints/Dialogues/EventData Structure (by ref)") (Narra :type Boolean) (Inspi :type Boolean))
  (returns (JustPlayed :type Boolean))
  (locals (PlayedThisTime :type Boolean))
  (bind _eventmanager (`self.EventManager`))
  (if Narra
    (bind _played_narra (`self.GetPlayed` EventData))
    (if (not _played_narra)
      (`/Game/Assets/Blueprints/Objects/EventManager.InteractWithEvent` _eventmanager EventData)
      (set `local.PlayedThisTime` true :!label _label))
    (elif Inspi
      (bind (_played_narra_2 _played_inspi) (`self.GetPlayed` EventData))
      (if (not _played_inspi)
        (`/Game/Assets/Blueprints/Objects/EventManager.InteractWithEvent` _eventmanager EventData)
        (goto _label)
        (else
          _))))
  (return (`local.PlayedThisTime`)))

(fn `SetCanPlay`
  (params (EventData :type "/Game/Assets/Blueprints/Dialogues/EventData Structure (by ref)") (CanPlay_Narra :type Boolean) (CanPlay_Inspi :type Boolean))
  (returns (`EventData ` :type "/Game/Assets/Blueprints/Dialogues/EventData Structure"))
  (locals (CanPlayNarra :type Boolean :default false) (CanPlayInspi :type Boolean :default false))
  (bind (_objectclass _canplay_narra _played_narra _audio_narra _subtitle_narra _canplay_inspi _played_inspi _audio_inspi _subtitle_inspi _idea_inspi) (break `/Game/Assets/Blueprints/Dialogues/EventData` EventData))
  (bind _canplaynarra (`local.CanPlayNarra`))
  (bind _canplayinspi (`local.CanPlayInspi`))
  (bind _eventdata (make `/Game/Assets/Blueprints/Dialogues/EventData` _objectclass _canplaynarra _played_narra _audio_narra _subtitle_narra _canplayinspi _played_inspi _audio_inspi _subtitle_inspi _idea_inspi))
  ;[1 1 1] Narra can play if narra not played
  (if (not _played_narra)
    (set `local.CanPlayNarra` CanPlay_Narra)
    (else
      (set `local.CanPlayNarra` false)))
  ;[1 1 1] Inspi can play if narra played and inspi not played
  (if (and _played_narra (not _played_inspi))
    (set `local.CanPlayInspi` CanPlay_Inspi)
    (else
      (set `local.CanPlayInspi` false)))
  (`|VariableSetRef` EventData _eventdata)
  (`/Game/Assets/Blueprints/Objects/EventManager.SetObject_CanPlay` (`self.EventManager`) _objectclass _canplaynarra _canplayinspi)
  (return _eventdata))

(fn `SetCanPlay_Array`
  (params (EventData_Array :type "Array of /Game/Assets/Blueprints/Dialogues/EventData Structure (by ref)") (CanPlay_Narra :type Boolean) (CanPlay_Inspi :type Boolean))
  (returns (NewEventData_Array :type "Array of /Game/Assets/Blueprints/Dialogues/EventData Structure"))
  (locals (NewEventDataArray :type "Array of /Game/Assets/Blueprints/Dialogues/EventData Structure"))
  (for _array_element EventData_Array
    (bind _eventdata_ (`self.SetCanPlay` _array_element CanPlay_Narra CanPlay_Inspi))
    (`KismetArrayLibrary.Array_Add` (`local.NewEventDataArray`) _eventdata_))
  (return (`local.NewEventDataArray`)))

(fn `SetPlayed`
  (params (EventData :type "/Game/Assets/Blueprints/Dialogues/EventData Structure") (Played_Narra :type Boolean) (Played_Inspi :type Boolean))
  (bind (_objectclass _canplay_narra _played_narra _audio_narra _subtitle_narra _canplay_inspi _played_inspi _audio_inspi _subtitle_inspi _idea_inspi) (break `/Game/Assets/Blueprints/Dialogues/EventData` EventData))
  (`|VariableSetRef` EventData (make `/Game/Assets/Blueprints/Dialogues/EventData` _objectclass _canplay_narra Played_Narra _audio_narra _subtitle_narra _canplay_inspi Played_Inspi _audio_inspi _subtitle_inspi _idea_inspi)))

(fn `UserConstructionScript`
  (bind _returnvalue (`GameplayStatics.GetActorOfClass` "/Game/Assets/Blueprints/Dialogues/DialogueManager.DialogueManager_C"))
  (set `self.DialogueManager` _returnvalue)
  (bind _returnvalue_2 (`GameplayStatics.GetActorOfClass` "/Game/Assets/Blueprints/Scenes/SceneManager.SceneManager_C"))
  (set `self.SceneManager` _returnvalue_2)
  (bind _returnvalue_3 (`GameplayStatics.GetActorOfClass` "/Game/Assets/Blueprints/Objects/EventManager.EventManager_C"))
  (set `self.EventManager` _returnvalue_3))