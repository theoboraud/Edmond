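; Scene 2 logic Blueprint that manages playable Narra and Inspi events for five objects (Stetson, Medocs, Foil, Apo, Helmet).
; BeginPlay loads each object's data from the Scene2_EventsData table.
; While no dialogue plays, Tick unlocks Narra first, then Inspi, and disables both once played.
; After at least three Inspi events, it locks all objects and sets EndTrigger, which later raises SceneManager's Scene 2 end trigger.
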(event `self.ReceiveBeginPlay`
  (`self.GetDataFromEvent`))

(event `self.ReceiveTick`
  (params (DeltaSeconds :type "Float (single-precision)"))
  ;[1 1 1] Start scene if initialized
  (if (`self.Initialized`)
    ;[1 1 1] Don't do anything if a dialogue is in play
    (bind _dialoguenotinplay (`self.DialogueNotInPlay`))
    (if _dialoguenotinplay
      ;[1 1 1] Stop here if scene 2 ended
      (if (`self.EndTrigger`)
        (set `/Game/Assets/Blueprints/Scenes/SceneManager.Scene2_EndTrigger` true (`self.SceneManager`))
        (else
          (`self.InitlializeCanPlay_AllObjects`
            (:`Exec `
              (bind _array (`self.GetAllObjects`))
              (bind _succeeded (`self.If at Least X Played` _array 3 false true))
              (if _succeeded
                (`self.SetCanPlay_AllObjects` false
                  (:`Exec `
                    (set `self.EndTrigger` true)))))))))))

(fn `GetAllObjects`
  (returns (Array :type "Array of /Game/Assets/Blueprints/Dialogues/EventData Structure"))
  (return (`|MakeArray` (`self.Stetson`) (`self.Medocs`) (`self.Foil`) (`self.Apo`) (`self.Helmet`))))

(fn `UserConstructionScript`
  (`parent.UserConstructionScript`))