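; Scene 3 controller that sequences dialogue interactions for four objects (Picture, Number, Sticker, Underwear) and signals when the scene ends.
; BeginPlay loads their events and the Intro from Scene3_EventsData by row name.
; Tick enables Narra lines, disabling played ones until Initialized, then runs the Intro check and per-object gating, where Inspi follows Narra.
; Once three Inspi lines have played, it locks all objects and sets SceneManager's Scene3EndTrigger after dialogue finishes.
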(event `self.ReceiveBeginPlay`
  (`self.GetDataFromEvent`))

(event `self.ReceiveTick`
  (params (DeltaSeconds :type "Float (single-precision)"))
  (bind _picture (`self.Picture`))
  (bind _number (`self.Number`))
  (bind _sticker (`self.Sticker`))
  (bind _underwear (`self.Underwear`))
  (if (not (`self.InitializedNarra`))
    (`self.SetCanPlay_AllObjects` true
      (:`Exec `
        (set `self.InitializedNarra` true)))
    (else
      ;[1 1 1] Start scene if initialized
      (if (`self.Initialized`)
        ;[1 1 1] Don't do anything if a dialogue is in play
        (bind _dialoguenotinplay (`self.DialogueNotInPlay`))
        (if _dialoguenotinplay
          ;[1 1 1] Stop here if scene 2 ended
          (if (`self.EndTrigger`)
            (set `/Game/Assets/Blueprints/Scenes/SceneManager.Scene3_EndTrigger` true (`self.SceneManager`))
            (else
              (bind _justplayed (`self.InteractionIfNotPlayed` (`self.Intro`) true))
              (if _justplayed
                (`self.InitlializeCanPlay_AllObjects`)
                (else
                  (bind _array (`self.GetAllObjects`))
                  (bind _succeeded (`self.If at Least X Played` _array 3 false true))
                  (if _succeeded
                    (`self.SetCanPlay_AllObjects` false
                      (:`Exec `
                        (set `self.EndTrigger` true)))))))))
        (else
          (bind _played_narra (`self.GetPlayed` _picture))
          (if _played_narra
            (`self.SetCanPlay` _picture))
          (bind _played_narra_2 (`self.GetPlayed` _number))
          (if _played_narra_2
            (`self.SetCanPlay` _number))
          (bind _played_narra_3 (`self.GetPlayed` _sticker))
          (if _played_narra_3
            (`self.SetCanPlay` _sticker))
          (bind _played_narra_4 (`self.GetPlayed` _underwear))
          (if _played_narra_4
            (`self.SetCanPlay` _underwear)))))))

(fn `GetAllObjects`
  (returns (Array :type "Array of /Game/Assets/Blueprints/Dialogues/EventData Structure"))
  (return (`|MakeArray` (`self.Number`) (`self.Sticker`) (`self.Underwear`) (`self.Picture`))))

(fn `UserConstructionScript`
  (`parent.UserConstructionScript`))