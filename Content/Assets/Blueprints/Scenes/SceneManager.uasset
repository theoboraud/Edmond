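; Scene manager actor that advances the game through five scenes plus a narrative scene.
; It caches the scene actors on BeginPlay, and Tick initializes the first scene whose end trigger is unset.
; InitializeScene flags each scene once and increments SceneCount, except for the narrative scene, which starts alongside Scene 2.
; GetAllActiveObjects appends objects from scenes reached so far to AllObjectData, but skips Scene 4.
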(event `self.ReceiveBeginPlay`
  (bind _returnvalue (`GameplayStatics.GetActorOfClass` "/Game/Assets/Blueprints/Scenes/Scene_1.Scene_1_C"))
  (set `self.Scene1` _returnvalue)
  (bind _returnvalue_2 (`GameplayStatics.GetActorOfClass` "/Game/Assets/Blueprints/Scenes/Scene_2.Scene_2_C"))
  (set `self.Scene2` _returnvalue_2)
  (bind _returnvalue_3 (`GameplayStatics.GetActorOfClass` "/Game/Assets/Blueprints/Scenes/Scene_3.Scene_3_C"))
  (set `self.Scene3` _returnvalue_3)
  (bind _returnvalue_4 (`GameplayStatics.GetActorOfClass` "/Game/Assets/Blueprints/Scenes/Scene_4.Scene_4_C"))
  (set `self.Scene4` _returnvalue_4)
  (bind _returnvalue_5 (`GameplayStatics.GetActorOfClass` "/Game/Assets/Blueprints/Scenes/Scene_5.Scene_5_C"))
  (set `self.Scene5` _returnvalue_5)
  (bind _returnvalue_6 (`GameplayStatics.GetActorOfClass` "/Game/Assets/Blueprints/Scenes/Scene_Narrative.Scene_Narrative_C"))
  (set `self.Scene_Narrative` _returnvalue_6))

(event `self.ReceiveTick`
  (params (DeltaSeconds :type "Float (single-precision)"))
  ;[1 1 1] Go to next scene if we triggered the current scene EndTrigger
  (if (not (`self.Scene1_EndTrigger`))
    (`self.InitializeScene` (`self.Scene1`)
      (:`Successfully initialized`
        (`KismetSystemLibrary.PrintString` (`KismetStringLibrary.Conv_IntToString` (`self.SceneCount`)))))
    (elif (not (`self.Scene2_EndTrigger`))
      (`self.InitializeScene` (`self.Scene2`)
        (:`Successfully initialized`
          (`KismetSystemLibrary.PrintString` (`KismetStringLibrary.Conv_IntToString` (`self.SceneCount`)))
          (`self.InitializeScene` (`self.Scene_Narrative`))))
      (elif (not (`self.Scene3_EndTrigger`))
        (`self.InitializeScene` (`self.Scene3`)
          (:`Successfully initialized`
            (`KismetSystemLibrary.PrintString` (`KismetStringLibrary.Conv_IntToString` (`self.SceneCount`)))))
        (elif (not (`self.Scene4_EndTrigger`))
          (`self.InitializeScene` (`self.Scene4`)
            (:`Successfully initialized`
              (`KismetSystemLibrary.PrintString` (`KismetStringLibrary.Conv_IntToString` (`self.SceneCount`)))))
          (elif (not (`self.Scene5_EndTrigger`))
            (`self.InitializeScene` (`self.Scene5`)
              (:`Successfully initialized`
                (`KismetSystemLibrary.PrintString` (`KismetStringLibrary.Conv_IntToString` (`self.SceneCount`)))))))))))

(fn `GetAllActiveObjects`
  (returns (Exec :type "Array of /Game/Assets/Blueprints/Dialogues/EventData Structure"))
  (locals (AllObjectData :type "Array of /Game/Assets/Blueprints/Dialogues/EventData Structure"))
  (bind _scenecount (`self.SceneCount`))
  (bind _allobjectdata (`local.AllObjectData`))
  (if (>= _scenecount 1)
    (bind _array (`/Game/Assets/Blueprints/Scenes/Scene_1.GetAllObjects` (`self.Scene1`)))
    (`KismetArrayLibrary.Array_Append` _allobjectdata _array)
    (if (>= _scenecount 2)
      (bind _array_2 (`/Game/Assets/Blueprints/Scenes/Scene_2.GetAllObjects` (`self.Scene2`)))
      (`KismetArrayLibrary.Array_Append` _allobjectdata _array_2)
      (bind _array_3 (`/Game/Assets/Blueprints/Scenes/Scene_Narrative.GetAllObjects` (`self.Scene_Narrative`)))
      (`KismetArrayLibrary.Array_Append` _allobjectdata _array_3)
      (if (>= _scenecount 3)
        (bind _array_4 (`/Game/Assets/Blueprints/Scenes/Scene_3.GetAllObjects` (`self.Scene3`)))
        (`KismetArrayLibrary.Array_Append` _allobjectdata _array_4)
        (if (>= _scenecount 4)
          (if (>= _scenecount 5)
            (bind _array_5 (`/Game/Assets/Blueprints/Scenes/Scene_5.GetAllObjects` (`self.Scene5`)))
            (`KismetArrayLibrary.Array_Append` _allobjectdata _array_5))))))
  (return (`local.AllObjectData`)))

(fn `UserConstructionScript`
  (bind _returnvalue (`GameplayStatics.GetActorOfClass` "/Game/Assets/Blueprints/Objects/EventManager.EventManager_C"))
  (set `self.EventManager` _returnvalue)
  (set `self.Scene1_EndTrigger` false)
  (set `self.Scene2_EndTrigger` false)
  (set `self.Scene3_EndTrigger` false)
  (set `self.Scene4_EndTrigger` false)
  (set `self.Scene5_EndTrigger` false))