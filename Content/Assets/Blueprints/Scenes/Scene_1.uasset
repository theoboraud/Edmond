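; Scene 1 controller that sequences the scene's dialogues and object interactions, loading its events from a data table at BeginPlay.
; While no dialogue plays, Tick checks played narrative and inspiration flags to unlock the Mask and four other objects.
; These flags trigger Intro, Call, two Assistant lines and the Outro, whose end trigger passes to SceneManager.
; A Coquelin impatience timer with waiting lines exists but is disconnected.
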(event `self.ReceiveBeginPlay`
  (`self.GetDataFromEvent`))

(event `self.ReceiveTick`
  (params (DeltaSeconds :type "Float (single-precision)"))
  (bind _endtrigger (`self.EndTrigger`))
  ;[1 1 1] Start scene if initialized
  (if (`self.Initialized`)
    ;[1 1 1] Don't do anything if a dialogue is in play
    (bind _dialoguenotinplay (`self.DialogueNotInPlay`))
    (if _dialoguenotinplay
      ;[1 1 1] Stop here if scene 1 ended
      (if _endtrigger
        (set `/Game/Assets/Blueprints/Scenes/SceneManager.Scene1_EndTrigger` _endtrigger (`self.SceneManager`))
        (else
          ;[1 1 1] Launch S1_Intro if not played already
          (`self.InteractionIfNotPlayed` (`self.Intro`) true)
          ;[1 1 1] The player must interact with the mask and at least 3 other objects
          (bind _played_narra (`self.GetPlayed` (`self.Mask`)))
          (if _played_narra
            (bind _array (`self.GetAllObjectsButMask`))
            (bind _succeeded (`self.If at Least X Played` _array 3 true))
            (if _succeeded
              ;[1 1 1] Launch S1_Call if not played already
              (bind _justplayed (`self.InteractionIfNotPlayed` (`self.Call`) true))
              (if _justplayed
                ;[1 1 1] Can't play other objects
                (`self.SetCanPlay_AllObjects` true
                  (:`Exec `
                    ;[1 1 1] Mask can be interacted inspi
                    (`self.SetCanPlay` (`self.Mask`) false true)
                    ;[1 1 1] Coquelin can become impatient
                    (set `self.CoquelinIsWaiting` true)))
                (else
                  ;[1 1 1] If mask interacted inspi, can interact with every other objects narratively interacted
                  (bind (_played_narra_2 _played_inspi) (`self.GetPlayed` (`self.Mask`)))
                  (if _played_inspi
                    ;[1 1 1] At first inspiration, launch S1_Assistant1
                    (bind _array_2 (`self.GetAllObjectsButMask`))
                    (bind _succeeded_2 (`self.If at Least X Played` _array_2 1 false true))
                    (if _succeeded_2
                      ;[1 1 1] Launch S1_Assistant1
                      (`self.InteractionIfNotPlayed` (`self.Assistant1`) true)
                      ;[1 1 1] At second inspiration, launch S1_Assistant2
                      (bind _array_3 (`self.GetAllObjectsButMask`))
                      (bind _succeeded_3 (`self.If at Least X Played` _array_3 2 false true))
                      (if _succeeded_3
                        ;[1 1 1] Launch S1_Assistant2
                        (`self.InteractionIfNotPlayed` (`self.Assistant2`) true)
                        ;[1 1 1] At third interaction, or third waiting, launch S1_Outro
                        (bind _array_4 (`self.GetAllObjectsButMask`))
                        (bind _succeeded_4 (`self.If at Least X Played` _array_4 3 false true))
                        (if _succeeded_4
                          (`self.InteractionIfNotPlayed` (`self.Outro`) true)
                          (set `self.CoquelinIsWaiting` false)
                          (set `self.EndTrigger` true)))
                      (else
                        ;[1 1 1] Other objects can be interacted inspi
                        (`self.SetCanPlay_AllObjects` false true))))))
              (else
                (`self.SetCanPlay_AllObjects` true false true)))
            (else
              (`self.SetCanPlay_AllObjects` true false true)))))
      (else
        (`self.ResetWaiting`)))))

(fn `GetAllObjects`
  (returns (Array :type "Array of /Game/Assets/Blueprints/Dialogues/EventData Structure"))
  (return (`|MakeArray` (`self.Mask`) (`self.Sword`) (`self.Penin`) (`self.Tower`) (`self.Ticket`))))

(fn `GetAllObjectsButMask`
  (returns (Array :type "Array of /Game/Assets/Blueprints/Dialogues/EventData Structure (by ref)"))
  (return (`|MakeArray` (`self.Sword`) (`self.Penin`) (`self.Tower`) (`self.Ticket`))))

(fn `UserConstructionScript`
  (`parent.UserConstructionScript`))